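; RapidMoveTo is a Behavior Tree task that moves an AI-controlled pawn toward the actor stored in the TargetToFollow blackboard key.
; On execute it casts the owner to MyAIController_BP, caches that reference for later runs, and runs AIMoveTo on the controlled pawn.
; A successful move finishes the task as failed, while a failed move or failed cast never calls FinishExecute.
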(event `self.ReceiveExecute`
  (params (OwnerActor :type "Actor Object Reference"))
  (if (not (!= (`self.AI_CON_Ref`) null))
    (bind _asmy_aicontroller_bp (cast `/Game/BluePrint/MyAIController_BP` OwnerActor))
    (set `self.AI_CON_Ref` _asmy_aicontroller_bp))
  (`|AIMoveTo` (`Controller.K2_GetPawn` (`self.AI_CON_Ref`)) (0.0 0.0 0.0) (`BTFunctionLibrary.GetBlackboardValueAsActor` (`self.TargetToFollow`))
    (:`OnSuccess`
      (`self.FinishExecute` false))))