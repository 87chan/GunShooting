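; HUD Blueprint that draws a custom mouse cursor and an animated gunshot effect on screen.
; Each DrawHUD pass centers the Cursor texture on the mouse position, then reads IsShot, ShotPos and AnimCount from MyPlayerController_BP.
; While IsShot is true, it draws the Gun texture around ShotPos as a five-frame horizontal sprite sheet, with AnimCount selecting the frame through the U offset.
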(event `self.ReceiveTick`
  (params (DeltaSeconds :type "Float (single-precision)")))

(event `self.ReceiveDrawHUD`
  (params (SizeX :type Integer) (SizeY :type Integer))
  (bind _returnvalue (`GameplayStatics.GetPlayerController` 0))
  (bind (_locationx _locationy) (`PlayerController.GetMousePosition` _returnvalue))
  (bind _returnvalue_2 (* (`self.EFF_WIDTH`) 0.5))
  (bind _returnvalue_3 (* (`self.CURSOR_LEN`) 0.5))
  (`|ExecutionSequence`
    (:`then_0`
      (`self.DrawTextureSimple` "/Game/Resource/Sprite/cursor.cursor" (- _locationx _returnvalue_3) (- _locationy _returnvalue_3) 1.0))
    (:`then_1`
      (bind _asmy_player_controller_bp (cast `/Game/BluePrint/MyPlayerController_BP` _returnvalue))
      (if (`/Game/BluePrint/MyPlayerController_BP.isShot` _asmy_player_controller_bp)
        (bind (_x _y) (`KismetMathLibrary.BreakVector2D` (`/Game/BluePrint/MyPlayerController_BP.shotPos` _asmy_player_controller_bp)))
        (`self.DrawTexture` "/Game/Resource/Sprite/gun.gun" (- _x _returnvalue_2) (- _y _returnvalue_2) 240.0 240.0 (* 0.2 (`KismetMathLibrary.Conv_IntToDouble` (`/Game/BluePrint/MyPlayerController_BP.animCount` _asmy_player_controller_bp))) 0.0 0.2 1.0)))))

(fn `UserConstructionScript`)